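; One-shot trigger zone that fires configurable scripted events when a BP_ThirdPersonCharacter first overlaps it.
; An IsActivated latch blocks repeats, then a sequence runs each action enabled by its flag.
; A timeline sets ObjectToMove's location straight to TargetPoint on each update, without interpolation.
; Quest updates, NPC dialogue and text cutscenes go to the player 0 character's HUD widget.
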(event EventBeginPlay)

(event Collision|EventActorBeginOverlap
  (params (OtherActor :type Actor%20Object%20Reference))
  (Utilities|Casting|CastToBP_ThirdPersonCharacter OtherActor)
  (if (not (Variables|Default|GetisActivated))
    (Variables|Default|SetisActivated true)
    (bind _asbp_third_person_character (Utilities|Casting|CastToBP_ThirdPersonCharacter (Game|GetPlayerCharacter 0)))
    (Utilities|FlowControl|Sequence
      (:then_0
        (if (Variables|MoveObject|GetMoveObject)
          (Timeline|MoveObjectTimeline Play
            (:Update
              (Transformation|SetActorLocation (Variables|MoveObject|GetObjectToMove) (Variables|MoveObject|GetTargetPoint) false false)))))
      (:then_1
        (if (Variables|QuestInfo|GetUpdateQuestInfo)
          (Default|UpdateQuestInfo (Variables|/Game/ThirdPerson/Blueprints/BP_ThirdPersonCharacter.BP_ThirdPersonCharacter_C|GetPlayerHUDWidget _asbp_third_person_character) (Variables|QuestInfo|GetQuestTitle) (Variables|QuestInfo|GetQuestGoal))))
      (:then_2
        (if (Variables|ShowDialogue|GetShowDialogue)
          (Default|ShowDialogue (Variables|/Game/ThirdPerson/Blueprints/BP_ThirdPersonCharacter.BP_ThirdPersonCharacter_C|GetPlayerHUDWidget _asbp_third_person_character) (Variables|ShowDialogue|GetNPC_Image) (Variables|ShowDialogue|GetNPC_Name) (Variables|ShowDialogue|GetNPC_Reply) (Variables|ShowDialogue|GetReplyDuration))))
      (:then_3
        (if (Variables|Cutscene|GetPlayCutscene)
          (Default|PlayCutscene (Variables|/Game/ThirdPerson/Blueprints/BP_ThirdPersonCharacter.BP_ThirdPersonCharacter_C|GetPlayerHUDWidget _asbp_third_person_character) (Variables|Cutscene|GetCutsceneText) (Variables|Cutscene|GetCutsceneDuration)))))))

(event EventTick
  (params (DeltaSeconds :type Float%20%28single-precision%29)))

(fn ConstructionScript)