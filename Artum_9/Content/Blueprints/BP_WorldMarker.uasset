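; BP_WorldMarker is an actor that shows an on-screen marker widget at its world location.
; It creates a WBP_WorldMarker widget for the first player on BeginPlay and removes it on EndPlay.
; Each Tick projects the actor's location to screen space to position the widget; the branch condition is always true, so the collapse path never runs.
; SetMarkerId stores an identifier that is not otherwise used here.
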(event EventBeginPlay
  (bind _returnvalue (UserInterface|CreateWidget "/Game/Widgets/WBP_WorldMarker.WBP_WorldMarker_C" (Game|GetPlayerController (Variables|/Script/Engine.Pawn|GetPlayerState (Game|GetPlayerCharacter 0)))))
  (bind _output_get (Variables|Default|SetMarkerWidget _returnvalue))
  (UserInterface|Viewport|AddtoViewport _output_get 0)
  (Class|UserWidget|SetDesiredSizeinViewport _output_get "(X=100.000000,Y=100.000000)"))

(event Collision|EventActorBeginOverlap
  (params (OtherActor :type Actor%20Object%20Reference)))

(event EventTick
  (params (DeltaSeconds :type Float%20%28single-precision%29))
  (if true
    (Class|UserWidget|SetPositioninViewport (stale EventBeginPlay _output_get) (.ScreenPosition (Class|GameplayStatics|ProjectWorldtoScreen (Game|GetPlayerController (Variables|/Script/Engine.Pawn|GetPlayerState (Game|GetPlayerCharacter 0))) (Transformation|GetActorLocation) false)) true)
    (else
      (Widget|SetVisibility (stale EventBeginPlay _output_get) "Collapsed"))))

(event EventEndPlay
  (params (EndPlayReason :type EEndPlayReason%20Enum :default "Destroyed"))
  (Widget|RemovefromParent (Variables|Default|GetMarkerWidget)))

(fn ConstructionScript)

(fn SetMarkerId
  (params (NewMarkerId :type String))
  (Variables|Default|SetMarkerId NewMarkerId))