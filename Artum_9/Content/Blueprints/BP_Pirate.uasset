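; BP_Pirate is a one-time interactable pirate that triggers a kill sequence on the player's HUD.
; A sphere overlap shows its Widget to the player until it is activated, and hides it when the player leaves.
; Interact latches IsActivated, hides the Widget, then uses IsChief to play either the chief or regular pirate kill sequence on the character's PlayerHUDWidget.
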(event OnComponentBeginOverlap(Sphere)
  (params (OverlappedComponent :type Primitive%20Component%20Object%20Reference) (OtherActor :type Actor%20Object%20Reference) (OtherComp :type Primitive%20Component%20Object%20Reference) (OtherBodyIndex :type Integer) (bFromSweep :type Boolean) (SweepResult :type Hit%20Result%20Structure%20%28by%20ref%29))
  (if (not (Variables|Default|GetisActivated))
    (if (== OtherActor (Game|GetPlayerCharacter 0))
      (Rendering|SetVisibility (Variables|Default|GetWidget) true false))))

(event OnComponentEndOverlap(Sphere)
  (params (OverlappedComponent :type Primitive%20Component%20Object%20Reference) (OtherActor :type Actor%20Object%20Reference) (OtherComp :type Primitive%20Component%20Object%20Reference) (OtherBodyIndex :type Integer))
  (if (== OtherActor (Game|GetPlayerCharacter 0))
    (Rendering|SetVisibility (Variables|Default|GetWidget) false false)))

(event EventInteract
  (if (not (Variables|Default|GetisActivated))
    (Variables|Default|SetisActivated true)
    (Rendering|SetVisibility (Variables|Default|GetWidget) false false)
    (bind _asbp_third_person_character (Utilities|Casting|CastToBP_ThirdPersonCharacter (Game|GetPlayerCharacter 0)))
    (if (Variables|Default|GetisChief)
      (Default|KillChiefSequence (Variables|/Game/ThirdPerson/Blueprints/BP_ThirdPersonCharacter.BP_ThirdPersonCharacter_C|GetPlayerHUDWidget _asbp_third_person_character))
      (else
        (Default|KillPiratesSequence (Variables|/Game/ThirdPerson/Blueprints/BP_ThirdPersonCharacter.BP_ThirdPersonCharacter_C|GetPlayerHUDWidget _asbp_third_person_character))))))

(fn ConstructionScript)