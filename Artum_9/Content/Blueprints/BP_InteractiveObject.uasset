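; One-shot interactable that shows a prompt widget while the player character is inside its sphere, until it is activated.
; On Interact it hides the prompt and runs whichever actions its boolean flags enable.
; Actions include sliding a target actor to a point by Timeline lerp, adding or removing markers through BP_ThirdPersonCharacter, and driving the player HUD for quest info, NPC dialogue and text cutscenes.
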(event OnComponentBeginOverlap(Sphere)
  (params (OverlappedComponent :type Primitive%20Component%20Object%20Reference) (OtherActor :type Actor%20Object%20Reference) (OtherComp :type Primitive%20Component%20Object%20Reference) (OtherBodyIndex :type Integer) (bFromSweep :type Boolean) (SweepResult :type Hit%20Result%20Structure%20%28by%20ref%29))
  (if (not (Variables|Default|GetisActivated))
    (if (== OtherActor (Game|GetPlayerCharacter 0))
      (Rendering|SetVisibility (Variables|Default|GetWidget) true false))))

(event OnComponentEndOverlap(Sphere)
  (params (OverlappedComponent :type Primitive%20Component%20Object%20Reference) (OtherActor :type Actor%20Object%20Reference) (OtherComp :type Primitive%20Component%20Object%20Reference) (OtherBodyIndex :type Integer))
  (if (== OtherActor (Game|GetPlayerCharacter 0))
    (Rendering|SetVisibility (Variables|Default|GetWidget) false false)))

(event EventInteract
  (if (not (Variables|Default|GetisActivated))
    (Variables|Default|SetisActivated true)
    (Rendering|SetVisibility (Variables|Default|GetWidget) false false)
    (bind _asbp_third_person_character (Utilities|Casting|CastToBP_ThirdPersonCharacter (Game|GetPlayerCharacter 0)))
    (Utilities|FlowControl|Sequence
      (:then_0
        (if (Variables|MoveObject|GetMoveObject)
          (bind _output_get (Variables|MoveObject|SetStartPoint (Transformation|GetActorLocation (Variables|MoveObject|GetObjectToMove))))
          (bind _floattrack (Timeline|Timeline PlayFromStart)
            (:Update
              (Transformation|SetActorLocation (Variables|MoveObject|GetObjectToMove) (Math|Vector|Lerp(Vector) _output_get (Variables|MoveObject|GetTargetPoint) _floattrack) false false)))))
      (:then_1
        (if (Variables|QuestInfo|GetUpdateQuestInfo)
          (Default|UpdateQuestInfo (Variables|/Game/ThirdPerson/Blueprints/BP_ThirdPersonCharacter.BP_ThirdPersonCharacter_C|GetPlayerHUDWidget _asbp_third_person_character) (Variables|QuestInfo|GetQuestTitle) (Variables|QuestInfo|GetQuestGoal))))
      (:then_2
        (if (Variables|ShowDialogue|GetShowDialogue)
          (Default|ShowDialogue (Variables|/Game/ThirdPerson/Blueprints/BP_ThirdPersonCharacter.BP_ThirdPersonCharacter_C|GetPlayerHUDWidget _asbp_third_person_character) (Variables|ShowDialogue|GetNPC_Image) (Variables|ShowDialogue|GetNPC_Name) (Variables|ShowDialogue|GetNPC_Reply) (Variables|ShowDialogue|GetReplyDuration))))
      (:then_3
        (if (Variables|Marker|GetCreateMarker)
          (Default|CreateMarker _asbp_third_person_character (Variables|Marker|GetSpawnMarkerLocation) (Variables|Marker|GetNewMarkerId))))
      (:then_4
        (if (Variables|Marker|GetRemoveMarker)
          (Default|RemoveMarker _asbp_third_person_character (Variables|Marker|GetRemoveMarkerId))))
      (:then_5
        (if (Variables|Cutscene|GetPlayCutscene)
          (Default|PlayCutscene (Variables|/Game/ThirdPerson/Blueprints/BP_ThirdPersonCharacter.BP_ThirdPersonCharacter_C|GetPlayerHUDWidget _asbp_third_person_character) (Variables|Cutscene|GetCutsceneText) (Variables|Cutscene|GetCutsceneDuration))))
      (:then_6
        (if (Variables|QuestInfo|GetHideQuestInfo)
          (Default|HideQuestInfo (Variables|/Game/ThirdPerson/Blueprints/BP_ThirdPersonCharacter.BP_ThirdPersonCharacter_C|GetPlayerHUDWidget _asbp_third_person_character)))))))

(fn ConstructionScript)